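; Charger enemy Blueprint that periodically dashes toward the player's position, overriding movement, touch and damage behavior.
; Tick accumulates time until the interval allows a charge, which locks a horizontal target at a set distance and draws a debug point.
; Swept constant-speed interpolation moves it there, blocking normal movement and using charge damage.
; Touching an actor mid-charge calls its Charged reaction and ends the dash; OnRepel's charge cancel is unwired.
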(event `self.ReceiveBeginPlay`
  (`parent.ReceiveBeginPlay`)
  (set `self.OriginSpeed` (`CharacterMovementComponent.MaxWalkSpeed` (`self.CharacterMovement`))))

(event `self.ReceiveTick`
  (params (DeltaSeconds :type "Float (single-precision)"))
  (`parent.ReceiveTick` DeltaSeconds)
  (`self.ChargeCheck` DeltaSeconds))

(fn `CanCharge`
  (returns (OutPut :type Boolean))
  (return (and (>= (`self.SumTime`) (`self.Interval`)) (not (`self.IsCharging`)) (not (`self.IsRepel`)))))

(fn `CanMove`
  (returns (OutPut :type Boolean))
  (return (and (not (`self.IsCharging`)) (not (`self.IsRepel`)))))

(fn `Charge`
  (bind _chargedis (`self.ChargeDis`))
  (bind (_returnvalue_x _returnvalue_y) (`KismetMathLibrary.BreakVector` (`KismetMathLibrary.GetDirectionUnitVector` (`self.K2_GetActorLocation`) (`self.K2_GetActorLocation` (`GameplayStatics.GetPlayerPawn` 0)))))
  (set `self.SumTime` 0.0)
  (set `self.IsCharging` true)
  (bind _output_get (set `self.ChargeTarget` (+ (`self.K2_GetActorLocation`) (* (`KismetMathLibrary.MakeVector` _returnvalue_x _returnvalue_y) (`KismetMathLibrary.MakeVector` _chargedis _chargedis)))))
  (`KismetSystemLibrary.DrawDebugPoint` _output_get 10.0 (struct :`R` 1.0 :`B` 0.064521 :`A` 1.0) 10.0))

(fn `ChargeCheck`
  (params (DeltaTime :type "Float (double-precision)"))
  (set `self.SumTime` (+ DeltaTime (`self.SumTime`)))
  (`|ExecutionSequence`
    (:`then_0`
      (if (`self.CanCharge`)
        (`self.Charge`)))
    (:`then_1`
      (if (`self.IsCharging`)
        (`self.TickCharge` (`local.DeltaTime`))))))

(fn `GetCurDamage`
  (returns (CurDamage :type "Float (double-precision)"))
  (return (select `bool` (`self.IsCharging`) :`false` (`self.BaseDamage`) :`true` (`self.ChargeDamage`))))

(fn `OnRepel`)

(fn `TickCharge`
  (params (DeltaTime :type "Float (double-precision)"))
  (`self.K2_SetActorLocation` (`KismetMathLibrary.VInterpTo_Constant` (`self.K2_GetActorLocation`) (`self.ChargeTarget`) (`local.DeltaTime`) (`self.ChargeSpeed`)) true)
  (if (< (`KismetMathLibrary.Vector_Distance` (`self.K2_GetActorLocation`) (`self.ChargeTarget`)) 1.0)
    (set `self.IsCharging` false)))

(fn `TouchEffect`
  (params (TouchActor :type "/Game/BluePrints/Player/BP_ThirdPersonCharacter Object Reference"))
  (if (`self.IsCharging`)
    (`/Game/BluePrints/Player/BP_ThirdPersonCharacter.Charged` TouchActor self 200.0)
    (set `self.IsCharging` false)))

(fn `UserConstructionScript`
  (`parent.UserConstructionScript`))