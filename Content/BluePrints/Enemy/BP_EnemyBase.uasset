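; Base enemy character providing knockback, timed slowdown, base damage and empty TouchEffect and OnRepel hooks.
; BeRepel sets a target that Tick moves toward with a swept constant-speed interpolation, while CanMove, false during knockback, is written to the Blackboard.
; SlowDown scales walk speed until its timer restores the original.
; Tick also periodically randomizes billboard visibility by a configurable rate.
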(event `self.ReceiveBeginPlay`
  (set `self.OriginSpeed` (`CharacterMovementComponent.MaxWalkSpeed` (`self.CharacterMovement`))))

(event `self.ReceiveTick`
  (params (DeltaSeconds :type "Float (single-precision)"))
  (bind _returnvalue (`AIBlueprintHelperLibrary.GetBlackboard` null))
  (`self.TickRepel` DeltaSeconds)
  (`self.SlowDownCheck` DeltaSeconds)
  (`self.UpdateBillBorad` DeltaSeconds)
  (`/Engine/EditorBlueprintResources/StandardMacros.IsValid` _returnvalue
    (:`Is Valid`
      (`BlackboardComponent.SetValueAsBool` _returnvalue (`self.CanMoveName`) (`self.CanMove`)))))

(fn `BeRepel`
  (params (RepelOffset :type "Vector Structure"))
  (set `self.RepelPos` (+ (`self.K2_GetActorLocation`) (`local.RepelOffset`)))
  (set `self.IsRepel` true)
  (`self.OnRepel`))

(fn `CanMove`
  (returns (OutPut :type Boolean))
  (return (not (`self.IsRepel`))))

(fn `GetCurDamage`
  (returns (CurDamage :type "Float (double-precision)"))
  (return (`self.BaseDamage`)))

(fn `OnRepel`)

(fn `SlowDown`
  (params (Percent :type "Float (double-precision)") (DurationTime :type "Float (double-precision)"))
  (set `self.SlowDownDurationTime` DurationTime)
  (set `self.SlowDownPastTime` 0.0)
  (set `CharacterMovementComponent.MaxWalkSpeed` (* (`self.OriginSpeed`) (- 1.0 (`local.Percent`))) (`self.CharacterMovement`))
  (set `self.IsSlowDown` true))

(fn `SlowDownCheck`
  (params (DeltaTime :type "Float (double-precision)"))
  (if (`self.IsSlowDown`)
    (bind _output_get (set `self.SlowDownPastTime` (+ (`self.SlowDownPastTime`) (`local.DeltaTime`))))
    (if (> _output_get (`self.SlowDownDurationTime`))
      (set `self.IsSlowDown` false)
      (set `CharacterMovementComponent.MaxWalkSpeed` (`self.OriginSpeed`) (`self.CharacterMovement`)))))

(fn `TickRepel`
  (params (DeltaTime :type "Float (double-precision)"))
  (if (`self.IsRepel`)
    (bind (_sweephitresult _returnvalue) (`self.K2_SetActorLocation` (`KismetMathLibrary.VInterpTo_Constant` (`self.K2_GetActorLocation`) (`self.RepelPos`) (`local.DeltaTime`) 800.0) true))
    (set `self.IsRepel` (and _returnvalue (> (`KismetMathLibrary.Vector_Distance` (`self.K2_GetActorLocation`) (`self.RepelPos`)) 0.0)))))

(fn `TouchEffect`
  (params (TouchActor :type "/Game/BluePrints/Player/BP_ThirdPersonCharacter Object Reference")))

(fn `UpdateBillBorad`
  (params (DeltaTime :type "Float (double-precision)"))
  (set `self.BillBoardPast` (+ (`self.BillBoardPast`) (`local.DeltaTime`)))
  (if (>= (`self.BillBoardPast`) (`self.BillBoardDuration`))
    (`SceneComponent.SetHiddenInGame` (`self.Billboard`) (< (`self.BillBoardRate`) (`KismetMathLibrary.RandomFloatInRange` 0.0 1.0)) false)
    (set `self.BillBoardPast` 0.0)))

(fn `UserConstructionScript`)