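; BP_Spit is the Spitter enemy's spit projectile component, which slows the player character it hits.
; Fly stores the Spitter, sets a target point at its FlyDistance along the direction to the given target, and enables movement.
; Tick moves it at constant FlySpeed with a swept move, passing the Spitter's slow settings to any BP_ThirdPersonCharacter hit.
; It destroys itself on a blocking hit or on reaching the target point.
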(event `self.ReceiveTick`
  (params (DeltaSeconds :type "Float (single-precision)"))
  (bind _spitter (`self.Spitter`))
  (if (`self.CanFly`)
    (`/Engine/EditorBlueprintResources/StandardMacros.IsValid` (`self.Spitter`)
      (:`Is Valid`
        (bind _sweephitresult (`self.K2_SetWorldLocation` (`KismetMathLibrary.VInterpTo_Constant` (`self.K2_GetComponentLocation`) (`self.TargetPos`) DeltaSeconds (`/Game/BluePrints/Enemy/Spitter/BP_Enemy_Spitter.FlySpeed` (`self.Spitter`))) true))
        (`|ExecutionSequence`
          (:`then_0`
            (bind (_bblockinghit _binitialoverlap _time _distance _location _impactpoint _normal _impactnormal _physmat _hitactor) (`GameplayStatics.BreakHitResult` _sweephitresult))
            (bind _asbp_third_person_character (cast `/Game/BluePrints/Player/BP_ThirdPersonCharacter` _hitactor))
            (`/Game/BluePrints/Player/BP_ThirdPersonCharacter.SlowDown` _asbp_third_person_character (`/Game/BluePrints/Enemy/Spitter/BP_Enemy_Spitter.DurationTime` _spitter) (`/Game/BluePrints/Enemy/Spitter/BP_Enemy_Spitter.Percent` _spitter)))
          (:`then_1`
            (if (or _bblockinghit (< (`KismetMathLibrary.Vector_Distance` (`self.K2_GetComponentLocation`) (`self.TargetPos`)) 1.0))
              (`self.K2_DestroyComponent`))))))))

(fn `Fly`
  (params (Target :type "Vector Structure") (Spitter :type "/Game/BluePrints/Enemy/Spitter/BP_Enemy_Spitter Object Reference"))
  (bind _flydistance (`/Game/BluePrints/Enemy/Spitter/BP_Enemy_Spitter.FlyDistance` (`self.Spitter`)))
  (set `self.Spitter` Spitter)
  (set `self.TargetPos` (+ (`self.K2_GetComponentLocation`) (* (`KismetMathLibrary.GetDirectionUnitVector` (`self.K2_GetComponentLocation`) (`local.Target`)) (`KismetMathLibrary.MakeVector` _flydistance _flydistance _flydistance))))
  (set `self.CanFly` true))