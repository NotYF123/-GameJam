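; Spitter enemy Blueprint that periodically fires spit at the player.
; Each Tick runs the parent logic, then TickSpitter adds delta time to a timer.
; When the timer reaches Interval, it resets, adds a new BP_Spit as a component at runtime and calls Fly with player 0's current pawn location.
; There are no range or line-of-sight checks in this Blueprint.
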(event `self.ReceiveTick`
  (params (DeltaSeconds :type "Float (single-precision)"))
  (`parent.ReceiveTick` DeltaSeconds)
  (`self.TickSpitter` DeltaSeconds))

(fn `TickSpitter`
  (params (DeltaTime :type "Float (double-precision)"))
  (set `self.SpitTime` (+ (`self.SpitTime`) (`local.DeltaTime`)))
  (if (>= (`self.SpitTime`) (`self.Interval`))
    (set `self.SpitTime` 0.0)
    (bind _returnvalue (`|AddComponentByClass` "/Game/BluePrints/Enemy/Spitter/BP_Spit.BP_Spit_C"))
    (`/Game/BluePrints/Enemy/Spitter/BP_Spit.Fly` _returnvalue (`self.K2_GetActorLocation` (`GameplayStatics.GetPlayerPawn` 0)) null)))

(fn `UserConstructionScript`
  (`parent.UserConstructionScript`))