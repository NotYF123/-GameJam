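; Enemy AI controller that runs the BT_Enemy behavior tree and feeds it the player as its target.
; On BeginPlay it starts the tree and seeds the blackboard with the player pawn, a CanMove flag set to true and the player's location as TargetPos.
; Every tick it overwrites TargetPos with the player's current location, with no perception or line-of-sight check in the controller.
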(event `self.ReceiveBeginPlay`
  (`self.RunBehaviorTree` "/Game/BluePrints/Enemy/AI/BT_Enemy.BT_Enemy")
  (`BlackboardComponent.SetValueAsObject` (`AIBlueprintHelperLibrary.GetBlackboard` null) (`self.Player`) (`GameplayStatics.GetPlayerPawn` 0))
  (`BlackboardComponent.SetValueAsBool` (`AIBlueprintHelperLibrary.GetBlackboard` null) (`self.CanMove`) true)
  (`BlackboardComponent.SetValueAsVector` (`AIBlueprintHelperLibrary.GetBlackboard` null) (`self.TargetPos`) (`self.K2_GetActorLocation` (`GameplayStatics.GetPlayerPawn` 0))))

(event `self.ReceiveTick`
  (params (DeltaSeconds :type "Float (single-precision)"))
  (`BlackboardComponent.SetValueAsVector` (`AIBlueprintHelperLibrary.GetBlackboard` null) (`self.TargetPos`) (`self.K2_GetActorLocation` (`GameplayStatics.GetPlayerPawn` 0))))

(fn `UserConstructionScript`)