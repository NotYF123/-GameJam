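; BP_ItemBase is a base item Blueprint that provides a time-based floating motion helper.
; Tick accumulates delta seconds into SumTime, which FloatingZ turns into a sine-wave value using a given frequency and amplitude, with the angle in degrees.
; The Blueprint only computes this offset and does not apply it to any transform itself.
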(event `self.ReceiveTick`
  (params (DeltaSeconds :type "Float (single-precision)"))
  (set `self.SumTime` (+ DeltaSeconds (`self.SumTime`))))

(fn `FloatingZ`
  (params (Frequency :type "Float (double-precision)" :default 3.0) (Amplitude :type "Float (double-precision)" :default 0.2))
  (returns (OutPut :type "Float (double-precision)"))
  (return (* (`KismetMathLibrary.DegSin` (* (`local.Frequency`) (`self.SumTime`))) (`local.Amplitude`))))

(fn `UserConstructionScript`)