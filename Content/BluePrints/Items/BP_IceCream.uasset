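; BP_IceCream is a touch pickup that slows enemies in an area behind the player who collects it.
; When the third-person character overlaps the capsule, Do moves a Box behind the player, sized by Width, and calls SlowDown on overlapping BP_EnemyBase actors.
; It then plays a Niagara effect above that area, hides the capsule, and destroys itself when the effect finishes.
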(event `self.ReceiveActorBeginOverlap`
  (params (OtherActor :type "Actor Object Reference")))

(event `self.ReceiveTick`
  (params (DeltaSeconds :type "Float (single-precision)"))
  (`parent.ReceiveTick` DeltaSeconds))

(event `self.Capsule.OnComponentBeginOverlap`
  (params (OverlappedComponent :type "PrimitiveComponent Object Reference") (OtherActor :type "Actor Object Reference") (OtherComp :type "PrimitiveComponent Object Reference") (OtherBodyIndex :type Integer) (bFromSweep :type Boolean) (SweepResult :type "HitResult Structure (by ref)"))
  (bind _asbp_third_person_character (cast `/Game/BluePrints/Player/BP_ThirdPersonCharacter` OtherActor))
  (add `NiagaraComponent.OnSystemFinished` (`self.Niagara`) (delegate `OnSystemFinished_Event`))
  (`self.Do` _asbp_third_person_character))

(event `OnSystemFinished_Event`
  (params (PSystem :type "NiagaraComponent Object Reference"))
  (`self.K2_DestroyActor`))

(fn `Do`
  (params (Player :type "/Game/BluePrints/Player/BP_ThirdPersonCharacter Object Reference"))
  (bind _niagara (`self.Niagara`))
  (bind _width (`self.Width`))
  (bind (_returnvalue_x _returnvalue_y _returnvalue_z) (`KismetMathLibrary.BreakVector` (`SceneComponent.K2_GetComponentLocation` (`self.Box`))))
  (bind _returnvalue (* (`self.Distance`) -1.0))
  (`SceneComponent.K2_SetWorldTransform` (`self.Box`) (`KismetMathLibrary.MakeTransform` (+ (`self.K2_GetActorLocation` Player) (* (`self.GetActorForwardVector` Player) (`KismetMathLibrary.MakeVector` _returnvalue _returnvalue -1.0))) (`self.K2_GetActorRotation` Player)) false false)
  (`BoxComponent.SetBoxExtent` (`self.Box`) (`KismetMathLibrary.MakeVector` _width _width 32.0) true)
  (for _array_element (`PrimitiveComponent.GetOverlappingActors` (`self.Box`) "/Game/BluePrints/Enemy/BP_EnemyBase.BP_EnemyBase_C")
    (bind _asbp_enemy_base (cast `/Game/BluePrints/Enemy/BP_EnemyBase` _array_element))
    (`/Game/BluePrints/Enemy/BP_EnemyBase.SlowDown` _asbp_enemy_base (`self.Percent`) (`self.DurationTime`)))
  (`SceneComponent.K2_SetWorldLocation` _niagara (`KismetMathLibrary.MakeVector` _returnvalue_x _returnvalue_y (+ _returnvalue_z 500.0)) false false)
  (`ActorComponent.Activate` _niagara false)
  (`SceneComponent.SetHiddenInGame` (`self.Capsule`) true true))

(fn `UserConstructionScript`
  (`parent.UserConstructionScript`))