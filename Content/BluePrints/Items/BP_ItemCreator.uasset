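; BP_ItemCreator is an item spawner actor that keeps one randomly chosen item spawned at its own transform.
; While no valid CreatedItem exists, Tick accumulates elapsed time until it reaches Interval.
; It then spawns a random class from ItemClass, stores it as CreatedItem and resets the timer, so the countdown resumes only after that item is gone.
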(event `self.ReceiveTick`
  (params (DeltaSeconds :type "Float (single-precision)"))
  (`/Engine/EditorBlueprintResources/StandardMacros.IsValid` (`self.CreatedItem`)
    (:`Is Not Valid`
      (set `self.PastTime` (+ DeltaSeconds (`self.PastTime`)))
      (if (>= (`self.PastTime`) (`self.Interval`))
        (bind _returnvalue (`|SpawnActorFromClass` (`KismetArrayLibrary.Array_Random` (`self.ItemClass`)) (`self.GetTransform`) "Undefined" "OverrideRootScale" null null))
        (set `self.CreatedItem` _returnvalue)
        (set `self.PastTime` 0.0)))))

(fn `UserConstructionScript`)